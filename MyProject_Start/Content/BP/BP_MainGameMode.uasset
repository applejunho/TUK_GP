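; BP_MainGameMode is the game mode that spawns and possesses the local player's character according to their selected role.
; On BeginPlay it reads LocalSelectedRole from MyGameInstance, spawning a killer character for role 1 and a tutorial character for any other value.
; Either pawn spawns at the first PlayerStart found and is possessed by player controller 0, with no handling for additional players.
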(event EventBeginPlay
  (bind _asmy_game_instance (Utilities|Casting|CastToMyGameInstance (Game|GetGameInstance)))
  (if (== (Variables|/Script/MyProject_Start.MyGameInstance|GetLocalSelectedRole _asmy_game_instance) 1)
    (bind _returnvalue (Actor|GetActorOfClass "/Script/Engine.PlayerStart"))
    (bind _returnvalue_2 (Game|SpawnActorfromClass "/Game/BP/BP_KillerCharacter.BP_KillerCharacter_C" (Transformation|GetActorTransform _returnvalue) "Undefined" "MultiplyWithRoot" 0 0))
    (Pawn|Possess (Game|GetPlayerController 0) _returnvalue_2)
    (else
      (bind _returnvalue_3 (Actor|GetActorOfClass "/Script/Engine.PlayerStart"))
      (bind _returnvalue_4 (Game|SpawnActorfromClass "/Game/BP/BP_TutorialCharacter.BP_TutorialCharacter_C" (Transformation|GetActorTransform _returnvalue_3) "Undefined" "MultiplyWithRoot" 0 0))
      (Pawn|Possess (Game|GetPlayerController 0) _returnvalue_4))))

(event EventTick
  (params (DeltaSeconds :type Float%20%28single-precision%29)))

(fn ConstructionScript)